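; Chaos field actor that progressively weakens internal cluster strain on rigid bodies inside a box, once triggered.
; CallTriggerActor enables and applies the field, which Tick also reapplies through a 0.2-second Delay.
; Each application subtracts box-aligned, scalable noise, multiplied by radial falloff and a decay amount, from the previous strain via a Return Results terminal.
; A box falloff culling field confines the effect.
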(event EventCallTriggerActor
  ;[0.9716 1 0.427] Internal Cluster Strain sets strain values across all rigid bodies with the field
  (bind _output_get (Variables|Default|Setactive true))
  (Class|FieldSystemComponent|ApplyPhysicsField (Variables|Field|GetFieldSystemComponent) _output_get "Field_InternalClusterStrain" 0 (Field|SetCullingField (Variables|Default|GetCullingField) (Field|SetBoxFalloff (Variables|Default|GetBoxFalloff) 1.0 0.0 1.0 0.0 (Transformation|GetWorldTransform (Variables|Default|GetBox)) "Field_Falloff_Linear") (Field|SetOperatorField (Variables|Default|GetOperatorField3) 1.0 (Field|SetOperatorField (Variables|Default|GetOperatorField2) 1.0 (Class|NoiseField|SetNoiseField (Variables|Default|GetNoiseField) (Variables|Default|GetnoiseMin) (Variables|Default|GetnoiseMax) (Math|Transform|MakeTransform (.location (stale EventTick _output_get)) (.rotation (stale EventTick _output_get)) (* (.scale (stale EventTick _output_get)) (Variables|Default|GetnoiseScaleMult)))) (Field|SetOperatorField (Variables|Default|GetOperatorField1) 1.0 (Class|UniformScalar|SetUniformScalar (Variables|Default|GetUniformScalar) (Variables|Default|GetdecayAmount)) (Field|SetRadialFalloff (Variables|Default|GetRadialFalloff) 1.0 0.0 1.0 0.0 (Variables|Default|GetfalloffRadius) (Transformation|GetWorldLocation (Variables|Default|GetBox)) "Field_Falloff_Linear") "Field_Multiply") "Field_Multiply") (Class|ReturnResultsTerminal|SetReturnResultsTerminal (Variables|Default|GetReturnResultsTerminal)) "Field_Substract") "Field_Culling_Outside")))

(event EventTick
  (params (DeltaSeconds :type Float%20%28single-precision%29))
  ;[1 1 1] Once activated, this field updates strain values on every tick
  (Utilities|FlowControl|Delay 0.2)
  ;[1 1 1] Noise
  ;;[1 1 1] Setting up noise field with controllable variables
  (bind _output_get (Variables|Default|SetTransformVar (Transformation|GetWorldTransform (Variables|Default|GetBox))))
  ;[0.9716 1 0.427] Internal Cluster Strain sets strain values across all rigid bodies with the field
  (Class|FieldSystemComponent|ApplyPhysicsField (Variables|Field|GetFieldSystemComponent) (stale EventCallTriggerActor _output_get) "Field_InternalClusterStrain" 0 (Field|SetCullingField (Variables|Default|GetCullingField) (Field|SetBoxFalloff (Variables|Default|GetBoxFalloff) 1.0 0.0 1.0 0.0 (Transformation|GetWorldTransform (Variables|Default|GetBox)) "Field_Falloff_Linear") (Field|SetOperatorField (Variables|Default|GetOperatorField3) 1.0 (Field|SetOperatorField (Variables|Default|GetOperatorField2) 1.0 (Class|NoiseField|SetNoiseField (Variables|Default|GetNoiseField) (Variables|Default|GetnoiseMin) (Variables|Default|GetnoiseMax) (Math|Transform|MakeTransform (.location _output_get) (.rotation _output_get) (* (.scale _output_get) (Variables|Default|GetnoiseScaleMult)))) (Field|SetOperatorField (Variables|Default|GetOperatorField1) 1.0 (Class|UniformScalar|SetUniformScalar (Variables|Default|GetUniformScalar) (Variables|Default|GetdecayAmount)) (Field|SetRadialFalloff (Variables|Default|GetRadialFalloff) 1.0 0.0 1.0 0.0 (Variables|Default|GetfalloffRadius) (Transformation|GetWorldLocation (Variables|Default|GetBox)) "Field_Falloff_Linear") "Field_Multiply") "Field_Multiply") (Class|ReturnResultsTerminal|SetReturnResultsTerminal (Variables|Default|GetReturnResultsTerminal)) "Field_Substract") "Field_Culling_Outside")))

(fn ConstructionScript)