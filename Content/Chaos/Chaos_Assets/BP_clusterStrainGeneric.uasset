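; Chaos field actor that applies external cluster strain to rigid bodies inside its box, for use with destruction.
; A box falloff node with no falloff takes the Box component's world transform and a Magnitude variable, and feeds the field system component.
; The field fires automatically after a short delay on BeginPlay.
; Toggle and CallTriggerActor fire the same field again after a briefer delay.
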(event EventToggle
  (params (On/off :type Boolean))
  (Utilities|FlowControl|Delay 0.3)
  ;[0.09621 1 0] This blueprint creates a box field and applies cluster strain to any rigid bodies inside
  ;;[1 1 1] Apply Physics Field nodes determine what attributes are affected by your field
  (Class|FieldSystemComponent|ApplyPhysicsField (Variables|Field|GetFieldSystemComponent) true "Field_ExternalClusterStrain" 0 (Field|SetBoxFalloff (Variables|Default|GetBoxFalloff) (Variables|Default|Getmagnitude) 0.0 1.0 0.0 (Transformation|GetWorldTransform (Variables|Default|GetBox)) "Field_FallOff_None")))

(event EventBeginPlay
  ;[0.09621 1 0] This blueprint creates a box field and applies cluster strain to any rigid bodies inside
  (Utilities|FlowControl|Delay 2.0)
  ;;[1 1 1] Apply Physics Field nodes determine what attributes are affected by your field
  (Class|FieldSystemComponent|ApplyPhysicsField (Variables|Field|GetFieldSystemComponent) true "Field_ExternalClusterStrain" 0 (Field|SetBoxFalloff (Variables|Default|GetBoxFalloff) (Variables|Default|Getmagnitude) 0.0 1.0 0.0 (Transformation|GetWorldTransform (Variables|Default|GetBox)) "Field_FallOff_None")))

(event EventTick
  (params (DeltaSeconds :type Float%20%28single-precision%29)))

(event EventCallTriggerActor
  (Utilities|FlowControl|Delay 0.3)
  ;[0.09621 1 0] This blueprint creates a box field and applies cluster strain to any rigid bodies inside
  ;;[1 1 1] Apply Physics Field nodes determine what attributes are affected by your field
  (Class|FieldSystemComponent|ApplyPhysicsField (Variables|Field|GetFieldSystemComponent) true "Field_ExternalClusterStrain" 0 (Field|SetBoxFalloff (Variables|Default|GetBoxFalloff) (Variables|Default|Getmagnitude) 0.0 1.0 0.0 (Transformation|GetWorldTransform (Variables|Default|GetBox)) "Field_FallOff_None")))

(fn ConstructionScript)